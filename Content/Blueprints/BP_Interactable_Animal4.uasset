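; Interactable farm chicken that wanders back and forth and produces eggs when fed.
; A looping timeline slides its trigger, plane and progress background out and back, pausing at each end.
; Interacting plays FMOD audio, then collects a ready egg through GM_Base, starts feeding if the sack is active, or sends a hunger message to the active HUD widget.
; Feeding runs a timeline that fills the progress bar and marks the egg ready.
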(event `self.ReceiveBeginPlay`
  (`parent.ReceiveBeginPlay`)
  (bind _asgm_base (cast `/Game/Blueprints/GM_Base` (`GameplayStatics.GetGameMode`)))
  (set `self.GameMode` _asgm_base)
  (bind _asbp_farm_hud (cast `/Game/Blueprints/BP_FarmHUD` (`PlayerController.GetHUD` (`GameplayStatics.GetPlayerController` 0))))
  (set `self.HUD` _asbp_farm_hud)
  (`KismetSystemLibrary.Delay` 2.0)
  (`self.Move`))

(event `Move`
  (bind (_direction _alpha) (`Timeline|MoveAnim` :!via `PlayFromStart` :!label _label)
    (:`Update`
      (set `self.Direction` _direction)
      (`SceneComponent.K2_SetRelativeLocation` (`self.Trigger`) (`KismetMathLibrary.VLerp` (0.0 0.0 48.207525) (`self.Location`) _alpha) false false)
      (`SceneComponent.K2_SetRelativeLocation` (`self.Plane`) (`KismetMathLibrary.VLerp` (0.0 0.0 48.207525) (`self.Location`) _alpha) false false)
      (`SceneComponent.K2_SetRelativeLocation` (`self.ProgressBK`) (`KismetMathLibrary.VLerp` (0.0 0.0 -33.747311) (-30.0 45.0 -33.747311) _alpha) false false))
    (:`Finished`
      (if (`|EnumEquality` (`self.Direction`) "Backward")
        (`KismetSystemLibrary.Delay` 2.0)
        (`self.Move`)
        (else
          (`KismetSystemLibrary.Delay` (`|GetArrayItem` (`self.WaitDuration`) (`KismetMathLibrary.RandomInteger` 1)))
          (goto _label :!via `Reverse`))))))

(event `self.Interact`
  (bind _returnvalue (`CommonActivatableWidgetContainerBase.GetActiveWidget` (`/Game/Blueprints/UI/WBP_Main.GameplayStack` (`/Game/Blueprints/BP_FarmHUD.MainWidgetRef` (`self.HUD`)))))
  (`FMODAudioComponent.Play` (`self.FMODAudio`))
  (if (`self.AnimalReady`)
    (`/Game/Blueprints/GM_Base.UpdateEggs` (`self.GameMode`) 1)
    (`KismetSystemLibrary.PrintString` "GotEgg")
    (set `self.AnimalReady` false)
    (`SceneComponent.SetRelativeScale3D` (`self.Progress`) (0.006983 0.0 0.946016))
    (elif (`/Game/Blueprints/GM_Base.SackActive` (`self.GameMode`))
      (if (not (`self.Eating`))
        (`self.Anim`))
      (elif (`KismetSystemLibrary.DoesImplementInterface` _returnvalue "/Game/Blueprints/Interfaces/BPI_Callable1.BPI_Callable1_C")
        (message `/Game/Blueprints/Interfaces/BPI_Callable1.Call` _returnvalue "Shnicken is hungry!")))))

(event `Anim`
  (set `self.AnimalReady` false)
  (set `self.Eating` true)
  (`TimelineComponent.SetPlayRate` (`self.ProgressAnim`) (`self.Duration`))
  (bind (_direction _alpha) (`Timeline|ProgressAnim` :!via `PlayFromStart`)
    (:`Update`
      (`SceneComponent.SetRelativeScale3D` (`self.Progress`) (`KismetMathLibrary.MakeVector` 0.006983 (`KismetMathLibrary.Lerp` 0.0 1.0 _alpha) 0.946016)))
    (:`Finished`
      (set `self.AnimalReady` true)
      (set `self.Eating` false))))

(fn `UserConstructionScript`
  (`parent.UserConstructionScript`))