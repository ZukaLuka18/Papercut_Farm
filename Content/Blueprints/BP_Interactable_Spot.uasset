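; Interactable farming spot where the player digs a hole, plants a seed, waters it through growth stages, then clears the grown plant.
; Interact checks the plant level and GM_Base tool/seed state, changing visibility and dynamic-material textures, with DoOnce guards per stage.
; Each planting or watering starts a timeline that shrinks a progress bar and blocks interaction until finished.
; Clearing the plant resets the guards and state for reuse.
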(event `self.ReceiveBeginPlay`
  (`parent.ReceiveBeginPlay`)
  (bind _asgm_base (cast `/Game/Blueprints/GM_Base` (`GameplayStatics.GetGameMode`)))
  (set `self.GameMode` _asgm_base))

(event `Countdown`
  (`TimelineComponent.SetPlayRate` (`self.CountdownAnim`) (`self.Duration`))
  (set `self.NeedWater` false)
  (bind (_direction _alpha) (`Timeline|CountdownAnim` :!via `PlayFromStart`)
    (:`Update`
      (`SceneComponent.SetRelativeScale3D` (`self.Progress`) (`KismetMathLibrary.MakeVector` 0.006983 (`KismetMathLibrary.Lerp` 0.056686 0.0 _alpha) 0.006983)))
    (:`Finished`
      (set `self.NeedWater` true))))

(event `/Game/Blueprints/Interfaces/BPI_Interact.Interact`
  (bind _gamemode (`self.GameMode`))
  (bind _gamemode_2 (`self.GameMode`))
  (if (`self.NeedWater`)
    (if (== (`self.PlantLV`) 4)
      (`SceneComponent.SetVisibility` (`self.Plant`) false false)
      (`SceneComponent.SetVisibility` (`self.Soil`) false false)
      (`self.Reset`)
      (set `self.PlantLV` 0)
      (set `self.Loch` false)
      (`MaterialInstanceDynamic.SetTextureParameterValue` (`self.PlantMaterial`) "Texture" "/Game/PNGS/Plant1.Plant1")
      (elif (and (`/Game/Blueprints/GM_Base.ShovelActive` _gamemode) (not (`self.Loch`)))
        (`/Engine/EditorBlueprintResources/StandardMacros.DoOnce` false :!label _label
          (:`Completed`
            (`MaterialInstanceDynamic.SetTextureParameterValue` (`self.BodenMaterial`) "Texture" "/Game/PNGS/BodenLoch.BodenLoch")
            (set `self.Loch` true)))
        (elif (and (and (> (`/Game/Blueprints/GM_Base.Seeds` _gamemode) 0) (`self.Loch`)) (== (`self.PlantLV`) 0))
          (`/Engine/EditorBlueprintResources/StandardMacros.DoOnce` false :!label _label_2
            (:`Completed`
              (`MaterialInstanceDynamic.SetTextureParameterValue` (`self.BodenMaterial`) "Texture" "/Game/PNGS/Boden.Boden")
              (`SceneComponent.SetVisibility` (`self.Soil`) true false)
              (set `self.PlantLV` 1)
              (`self.Countdown`)
              (set `/Game/Blueprints/GM_Base.Seeds` (- (`/Game/Blueprints/GM_Base.Seeds` _gamemode_2) 1) _gamemode_2)))
          (elif (and (`/Game/Blueprints/GM_Base.CaneActive` _gamemode) (== (`self.PlantLV`) 1))
            (`/Engine/EditorBlueprintResources/StandardMacros.DoOnce` false :!label _label_3
              (:`Completed`
                (`SceneComponent.SetVisibility` (`self.Plant`) true false)
                (set `self.PlantLV` 2)
                (`self.Countdown`)))
            (elif (and (`/Game/Blueprints/GM_Base.CaneActive` _gamemode) (== (`self.PlantLV`) 2))
              (`/Engine/EditorBlueprintResources/StandardMacros.DoOnce` false :!label _label_4
                (:`Completed`
                  (`MaterialInstanceDynamic.SetTextureParameterValue` (`self.PlantMaterial`) "Texture" "/Game/PNGS/Plant2.Plant2")
                  (set `self.PlantLV` 3)
                  (`self.Countdown`)))
              (elif (and (`/Game/Blueprints/GM_Base.CaneActive` _gamemode) (== (`self.PlantLV`) 3))
                (`/Engine/EditorBlueprintResources/StandardMacros.DoOnce` false :!label _label_5
                  (:`Completed`
                    (`MaterialInstanceDynamic.SetTextureParameterValue` (`self.PlantMaterial`) "Texture" "/Game/PNGS/Plant3.Plant3")
                    (set `self.PlantLV` 4)
                    (`self.Countdown`)))))))))))

(event `Reset`
  (`|ExecutionSequence`
    (:`then_0`
      (goto _label :!via `Reset`))
    (:`then_1`
      (goto _label_2 :!via `Reset`))
    (:`then_2`
      (goto _label_3 :!via `Reset`))
    (:`then_3`
      (goto _label_4 :!via `Reset`))
    (:`then_4`
      (goto _label_5 :!via `Reset`))))

(fn `UserConstructionScript`
  (bind _returnvalue (`PrimitiveComponent.CreateDynamicMaterialInstance` (`self.Boden`) 0 "/Game/Material/M_Texture_Spot.M_Texture_Spot" "None"))
  (set `self.BodenMaterial` _returnvalue)
  (bind _returnvalue_2 (`PrimitiveComponent.CreateDynamicMaterialInstance` (`self.Plant`) 0 "/Game/Material/M_Texture_Plant.M_Texture_Plant" "None"))
  (set `self.PlantMaterial` _returnvalue_2)
  (`parent.UserConstructionScript`))