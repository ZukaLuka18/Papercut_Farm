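; Quest manager component that queues quests and shows an accepted-quest widget for the quest at the front of the queue.
; SetUp stores the widget stack, and AddQuestToQueue adds quests uniquely, calling ShowQuest only when the queue length is one.
; ShowQuest pushes WBP_AcceptedQuest onto that stack and sets it up with the first entry; nothing here removes or advances queued quests.
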(event `SetUp`
  (params (Stack :type "CommonActivatableWidgetStack Object Reference"))
  (set `self.Stack` Stack))

(event `AddQuestToQueue`
  (params (Quest :type "/Game/Blueprints/Data/STRUCT_Quest Structure"))
  (bind _questqueue (`self.QuestQueue`))
  (`KismetArrayLibrary.Array_AddUnique` _questqueue Quest)
  (if (== (`KismetArrayLibrary.Array_Length` _questqueue) 1)
    (`self.ShowQuest`)))

(event `ShowQuest`
  (bind _returnvalue (`CommonActivatableWidgetContainerBase.BP_AddWidget` (`self.Stack`) "/Game/Blueprints/UI/WBP_AcceptedQuest.WBP_AcceptedQuest_C"))
  (`/Game/Blueprints/UI/WBP_AcceptedQuest.Setup` _returnvalue (`|GetArrayItem` (`self.QuestQueue`))))