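; BP_Interactable_Tools_Cane is an interactable tool that toggles the cane shown on the player.
; Interact first runs CheckForShovel, which hides the player's Shovel and Sack, clears their GameMode active flags and resets Interacted if either is visible.
; It then uses the Interacted flag to show or hide the player's Cane and sets GameMode.CaneActive to match.
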(event `/Game/Blueprints/Interfaces/BPI_Interact.Interact`
  (bind _gamemode (`self.GameMode`))
  (bind _cane (`/Game/Blueprints/BP_Player.Cane` (`self.Player`)))
  (`self.CheckForShovel`)
  (if (`self.Interacted`)
    (`SceneComponent.SetVisibility` _cane false false)
    (set `self.Interacted` false)
    (set `/Game/Blueprints/GM_Base.CaneActive` false _gamemode)
    (else
      (`SceneComponent.SetVisibility` _cane true false)
      (set `self.Interacted` true)
      (set `/Game/Blueprints/GM_Base.CaneActive` true _gamemode))))

(event `CheckForShovel`
  (bind _player (`self.Player`))
  (bind _gamemode (`self.GameMode`))
  (bind _shovel (`/Game/Blueprints/BP_Player.Shovel` _player))
  (bind _sack (`/Game/Blueprints/BP_Player.Sack` _player))
  (if (or (`SceneComponent.IsVisible` _sack) (`SceneComponent.IsVisible` _shovel))
    (`|ExecutionSequence`
      (:`then_0`
        (`SceneComponent.SetVisibility` _shovel false false)
        (set `/Game/Blueprints/GM_Base.ShovelActive` false _gamemode)
        (set `self.Interacted` false))
      (:`then_1`
        (`SceneComponent.SetVisibility` _sack false false)
        (set `/Game/Blueprints/GM_Base.SackActive` false _gamemode)
        (set `self.Interacted` false)))))

(fn `UserConstructionScript`
  (`parent.UserConstructionScript`))