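; Base game mode that tracks farm product counts and checks them against quests of up to three orders.
; BeginPlay builds Products from DT_Quests Order1 values, and CheckFirstOrder stores each order's index in that list, which selects the counter to compare.
; Counter updates recheck active orders, setting CanComit once required ones are met.
; UpdateEggs adds to Milk, and CheckSecondOrder only prints debug text.
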(event `UpdateSting`
  (params (Amount :type Integer))
  (set `self.Stingsquach` (+ (`self.Stingsquach`) Amount))
  (`self.CheckAll`))

(event `UpdateMilk`
  (params (Amount :type Integer))
  (set `self.Milk` (+ (`self.Milk`) Amount))
  (`self.CheckAll`))

(event `UpdatePlants`
  (params (Amount :type Integer))
  (set `self.Trunkblume` (+ (`self.Trunkblume`) Amount))
  (`self.CheckAll`))

(event `CorrectAmount_1`
  (bind _amountorder1 (`self.AmountOrder1`))
  (bind _foundorder1 (`self.FoundOrder1`))
  (`|ExecutionSequence`
    (:`then_0`
      (if (== _foundorder1 0)
        (set `self.ItsTrunk` true)
        (if (>= (`self.Trunkblume`) _amountorder1)
          (set `self.Correct1` true :!label _label)
          (`self.CheckQuest`))))
    (:`then_1`
      (if (== _foundorder1 1)
        (set `self.ItsSting` true)
        (if (>= (`self.Stingsquach`) _amountorder1)
          (goto _label))))
    (:`then_2`
      (if (== _foundorder1 2)
        (set `self.ItsMilk` true)
        (if (>= (`self.Milk`) _amountorder1)
          (goto _label))))
    (:`then_3`
      (if (== _foundorder1 3)
        (set `self.ItsGoat` true)
        (if (>= (`self.Goat`) _amountorder1)
          (goto _label))))))

(event `UpdateEggs`
  (params (Amount :type Integer))
  (set `self.Milk` (+ (`self.Milk`) Amount))
  (`self.CheckAll`))

(event `CheckAll`
  (if (`self.QuestOn`)
    (`self.CorrectAmount_1`)
    (`self.AmountCorrect_2`)
    (`self.AmountCorrect_3`)))

(event `self.ReceiveBeginPlay`
  (bind _outrownames (`DataTableFunctionLibrary.GetDataTableRowNames` "/Game/Blueprints/Data/DT_Quests.DT_Quests"))
  (for _array_element _outrownames
    (bind _returnvalue (`|GetDataTableRow` "/Game/Blueprints/Data/DT_Quests.DT_Quests" _array_element)
      (:`then`
        (`KismetArrayLibrary.Array_AddUnique` (`self.Products`) (`KismetTextLibrary.Conv_TextToString` (`.Order_1_10_A19E410B4CADC127A528EAA90B493097` (break `/Game/Blueprints/Data/STRUCT_Quest` _returnvalue))))))))

(event `CheckQuest`
  (if (`self.Correct1`)
    (if (`self.NeedCorrect2`)
      (if (`self.Correct2`)
        (if (`self.NeedCorrect3`)
          (if (`self.Correct3`)
            (set `self.CanComit` true)
            (`KismetSystemLibrary.PrintString` "Win"))
          (else
            (set `self.CanComit` true)
            (`KismetSystemLibrary.PrintString` "Win"))))
      (else
        (set `self.CanComit` true)
        (`KismetSystemLibrary.PrintString` "Win")))))

(event `AmountCorrect_2`
  (bind _foundorder2 (`self.FoundOrder2`))
  (bind _amountorder2 (`self.AmountOrder2`))
  (if (`self.NeedCorrect2`)
    (`|ExecutionSequence`
      (:`then_0`
        (if (== _foundorder2 0)
          (set `self.ItsTrunk` true)
          (if (>= (`self.Trunkblume`) _amountorder2)
            (set `self.Correct2` true :!label _label_2)
            (`self.CheckQuest`))))
      (:`then_1`
        (if (== _foundorder2 1)
          (set `self.ItsSting` true)
          (if (>= (`self.Stingsquach`) _amountorder2)
            (goto _label_2))))
      (:`then_2`
        (if (== _foundorder2 2)
          (set `self.ItsMilk` true)
          (if (>= (`self.Milk`) _amountorder2)
            (goto _label_2))))
      (:`then_3`
        (if (== _foundorder2 3)
          (set `self.ItsGoat` true)
          (if (>= (`self.Goat`) _amountorder2)
            (goto _label_2)))))))

(event `AmountCorrect_3`
  (bind _foundorder3 (`self.FoundOrder3`))
  (bind _amountorder3 (`self.AmountOrder3`))
  (if (`self.NeedCorrect3`)
    (`|ExecutionSequence`
      (:`then_0`
        (if (== _foundorder3 0)
          (set `self.ItsTrunk` true)
          (if (>= (`self.Trunkblume`) _amountorder3)
            (set `self.Correct3` true :!label _label_3)
            (`self.CheckQuest`))))
      (:`then_1`
        (if (== _foundorder3 1)
          (set `self.ItsSting` true)
          (if (>= (`self.Stingsquach`) _amountorder3)
            (goto _label_3))))
      (:`then_2`
        (if (== _foundorder3 2)
          (set `self.ItsMilk` true)
          (if (>= (`self.Milk`) _amountorder3)
            (goto _label_3))))
      (:`then_3`
        (if (== _foundorder3 3)
          (set `self.ItsGoat` true)
          (if (>= (`self.Goat`) _amountorder3)
            (goto _label_3)))))))

(event `CheckFirstOrder`
  (params (Order1 :type String) (Amount1 :type Integer) (Order2 :type "String (by ref)") (Amount2 :type Integer) (Order3 :type "String (by ref)") (Amount3 :type Integer))
  (bind _products (`self.Products`))
  (set `self.QuestOn` true)
  (`|ExecutionSequence`
    (:`then_0`
      (set `self.FoundOrder1` (`KismetArrayLibrary.Array_Find` _products Order1))
      (set `self.AmountOrder1` Amount1)
      (`self.CheckAll`))
    (:`then_1`
      (if (`KismetStringLibrary.IsEmpty` Order2)
        (set `self.NeedCorrect2` false)
        (else
          (set `self.FoundOrder2` (`KismetArrayLibrary.Array_Find` _products Order2))
          (set `self.AmountOrder2` Amount2)
          (`self.CheckAll`))))
    (:`then_2`
      (if (`KismetStringLibrary.IsEmpty` Order3)
        (set `self.NeedCorrect3` false)
        (else
          (set `self.FoundOrder3` (`KismetArrayLibrary.Array_Find` _products Order3))
          (set `self.AmountOrder3` Amount3)
          (`self.CheckAll`))))))

(event `CheckSecondOrder`
  (params (Order1 :type String) (Amount1 :type Integer) (Order2 :type "String (by ref)") (Amount2 :type Integer) (Order3 :type "String (by ref)") (Amount3 :type Integer))
  (bind _products (`self.Products`))
  (`|ExecutionSequence`
    (:`then_0`
      (if (>= (select `int` (`KismetArrayLibrary.Array_Find` _products Order1) :`0` (`self.Trunkblume`) :`1` (`self.Stingsquach`) :`2` 0 :`3` 0 :`4` 0 :`5` 0 :`6` 0 :`7` 0 :`8` (`self.Eggs`)) Amount1)
        (`KismetSystemLibrary.PrintString` "Hello")))
    (:`then_1`
      (if (`KismetStringLibrary.IsEmpty` Order2)
        _
        (elif (>= (select `int` (`KismetArrayLibrary.Array_Find` _products Order2) :`0` (`self.Trunkblume`) :`1` (`self.Stingsquach`) :`2` 0 :`3` 0 :`4` 0 :`5` 0 :`6` 0 :`7` 0 :`8` (`self.Eggs`)) Amount2)
          (`KismetSystemLibrary.PrintString` "Hello"))))
    (:`then_2`
      (if (`KismetStringLibrary.IsEmpty` Order3)
        _
        (elif (>= (select `int` (`KismetArrayLibrary.Array_Find` _products Order3) :`0` (`self.Trunkblume`) :`1` (`self.Stingsquach`) :`2` 0 :`3` 0 :`4` 0 :`5` 0 :`6` 0 :`7` 0 :`8` (`self.Eggs`)) Amount3)
          (`KismetSystemLibrary.PrintString` "Hello"))))))

(fn `UserConstructionScript`)