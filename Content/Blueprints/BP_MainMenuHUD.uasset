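; Main menu HUD Blueprint that creates the WBP_Main1 root widget on BeginPlay, adds it to the viewport and keeps a reference to it.
; PushToGameplayStack adds widgets to the root's MenuStack, and BacktoGameplayStack removes that stack's active widget, despite both names referring to gameplay.
; PushToMenuStack and PushToQuestBoardStack are empty stubs.
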(event `self.ReceiveBeginPlay`
  (bind _returnvalue (`|CreateWidget` "/Game/Blueprints/UI/WBP_Main1.WBP_Main1_C"))
  (`UserWidget.AddToViewport` _returnvalue 0)
  (set `self.Ref` _returnvalue))

(event `/Game/Blueprints/Interfaces/BPI_PushWidgets.BackToGameplayStack`
  (bind _menustack (`/Game/Blueprints/UI/WBP_Main1.MenuStack` (`self.Ref`)))
  (`CommonActivatableWidgetContainerBase.RemoveWidget` _menustack (`CommonActivatableWidgetContainerBase.GetActiveWidget` _menustack)))

(fn `PushToGameplayStack`
  (params (Widget :type "CommonActivatableWidget Class Reference"))
  (returns (PushedWidget :type "CommonActivatableWidget Object Reference"))
  (bind _returnvalue (`CommonActivatableWidgetContainerBase.BP_AddWidget` (`/Game/Blueprints/UI/WBP_Main1.MenuStack` (`self.Ref`)) Widget))
  (return _returnvalue))

(fn `PushToMenuStack`
  (params (Widget :type "CommonActivatableWidget Class Reference"))
  (returns (PushedWidget :type "CommonActivatableWidget Object Reference"))
  (return null))

(fn `PushToQuestBoardStack`
  (params (Widget :type "CommonActivatableWidget Class Reference"))
  (returns (PushedWidget :type "CommonActivatableWidget Object Reference"))
  (return null))

(fn `UserConstructionScript`)