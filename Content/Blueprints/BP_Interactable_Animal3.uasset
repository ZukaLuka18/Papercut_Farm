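; Interactable animal that shuttles back and forth and plays the Schnicken audio event in 2D when interacted with.
; The MoveAnim timeline lerps the Plane, ProgressBK and Trigger components between relative origin and Location, alternately restarting and reversing after a delay from WaitDuration.
; The delay index uses RandomInteger(1), so it always picks the first entry.
; BeginPlay starts the loop and caches the GM_Base game mode.
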(event `self.ReceiveBeginPlay`
  (`parent.ReceiveBeginPlay`)
  (`self.Move`)
  (bind _asgm_base (cast `/Game/Blueprints/GM_Base` (`GameplayStatics.GetGameMode`)))
  (set `self.GameMode` _asgm_base))

(event `Move`
  (bind (_direction _alpha) (`Timeline|MoveAnim` :!via `PlayFromStart` :!label _label)
    (:`Update`
      (set `self.Direction` _direction)
      (`|ExecutionSequence`
        (:`then_1`
          (`SceneComponent.K2_SetRelativeLocation` (`self.Plane`) (`KismetMathLibrary.VLerp` (0.0 0.0 0.0) (`self.Location`) _alpha) false false)
          (`SceneComponent.K2_SetRelativeLocation` (`self.ProgressBK`) (`KismetMathLibrary.VLerp` (0.0 0.0 0.0) (`self.Location`) _alpha) false false)
          (`SceneComponent.K2_SetRelativeLocation` (`self.Trigger`) (`KismetMathLibrary.VLerp` (0.0 0.0 0.0) (`self.Location`) _alpha) false false))))
    (:`Finished`
      (if (`|EnumEquality` (`self.Direction`) "Backward")
        (`KismetSystemLibrary.Delay` (`|GetArrayItem` (`self.WaitDuration`) (`KismetMathLibrary.RandomInteger` 1)))
        (`self.Move`)
        (else
          (`KismetSystemLibrary.Delay` (`|GetArrayItem` (`self.WaitDuration`) (`KismetMathLibrary.RandomInteger` 1)))
          (goto _label :!via `Reverse`))))))

(event `/Game/Blueprints/Interfaces/BPI_Interact.Interact`
  (`FMODBlueprintStatics.PlayEvent2D` "/Game/FMOD/Events/Schnicken.Schnicken"))

(fn `UserConstructionScript`
  (`parent.UserConstructionScript`))