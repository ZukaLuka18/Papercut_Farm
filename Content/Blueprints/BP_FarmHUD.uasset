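; Farm HUD that owns the main UI widget and serves as the entry point for widget stack navigation and quest display.
; On BeginPlay it adds WBP_Main to the viewport and hands its gameplay stack to the quest manager component.
; Helper functions push widgets onto the gameplay or quest board stack, and matching back events remove the active one.
; ShowQuest forwards quests to the quest manager's queue.
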(event `self.ReceiveBeginPlay`
  ;[1 1 1] push mainwidget to gameplaystack
  (bind _returnvalue (`|CreateWidget` "/Game/Blueprints/UI/WBP_Main.WBP_Main_C"))
  (`UserWidget.AddToViewport` _returnvalue 0)
  (bind _output_get (set `self.MainWidgetRef` _returnvalue))
  (`/Game/Blueprints/Components/BP_QuestManagerComp.SetUp` (`self.BP_QuestManagerComp`) (`/Game/Blueprints/UI/WBP_Main.GameplayStack` _output_get)))

(event `/Game/Blueprints/Interfaces/BPI_PushWidgets.BackToGameplayStack`
  (bind _gameplaystack (`/Game/Blueprints/UI/WBP_Main.GameplayStack` (`self.MainWidgetRef`)))
  ;[1 1 1] remove widget
  (`CommonActivatableWidgetContainerBase.RemoveWidget` _gameplaystack (`CommonActivatableWidgetContainerBase.GetActiveWidget` _gameplaystack)))

(event `/Game/Blueprints/Interfaces/BPI_PushWidgets.BackToQuestBoardStack`
  (bind _questboardstack (`/Game/Blueprints/UI/WBP_Main.QuestBoardStack` (`self.MainWidgetRef`)))
  ;[1 1 1] remove quest board widget
  (`CommonActivatableWidgetContainerBase.RemoveWidget` _questboardstack (`CommonActivatableWidgetContainerBase.GetActiveWidget` _questboardstack)))

(event `/Game/Blueprints/Interfaces/BPI_PushWidgets.ShowQuest`
  (params (Quest :type "/Game/Blueprints/Data/STRUCT_Quest Structure"))
  ;[1 1 1] AddQuest
  (`/Game/Blueprints/Components/BP_QuestManagerComp.AddQuestToQueue` (`self.BP_QuestManagerComp`) Quest))

(fn `PushToGameplayStack`
  (params (Widget :type "CommonActivatableWidget Class Reference"))
  (returns (PushedWidget :type "CommonActivatableWidget Object Reference"))
  (bind _returnvalue (`CommonActivatableWidgetContainerBase.BP_AddWidget` (`/Game/Blueprints/UI/WBP_Main.GameplayStack` (`self.MainWidgetRef`)) Widget))
  (return _returnvalue))

(fn `PushToQuestBoardStack`
  (params (Widget :type "CommonActivatableWidget Class Reference"))
  (returns (PushedWidget :type "CommonActivatableWidget Object Reference"))
  (bind _returnvalue (`CommonActivatableWidgetContainerBase.BP_AddWidget` (`/Game/Blueprints/UI/WBP_Main.QuestBoardStack` (`self.MainWidgetRef`)) Widget))
  (return _returnvalue))

(fn `UserConstructionScript`)