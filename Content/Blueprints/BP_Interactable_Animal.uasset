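; BP_Interactable_Animal is an interactable animal that moves back and forth and gives milk when ready.
; A timeline lerps its Trigger and Plane between relative origin and a Location entry, pausing at each end before reversing or replaying.
; Random indices use RandomInteger(1), so only the first Location and WaitDuration entries are used.
; Interacting adds milk through GM_Base, then blocks further milking for Duration.
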(event `self.ReceiveBeginPlay`
  (`parent.ReceiveBeginPlay`)
  (`self.Move`)
  (bind _asgm_base (cast `/Game/Blueprints/GM_Base` (`GameplayStatics.GetGameMode`)))
  (set `self.GameMode` _asgm_base))

(event `Move`
  (bind (_direction _alpha) (`Timeline|MoveAnim` :!via `PlayFromStart` :!label _label)
    (:`Update`
      (set `self.Direction` _direction)
      (`SceneComponent.K2_SetRelativeLocation` (`self.Trigger`) (`KismetMathLibrary.VLerp` (0.0 0.0 0.0) (`|GetArrayItem` (`self.Location`) (`KismetMathLibrary.RandomInteger` 1)) _alpha) false false)
      (`SceneComponent.K2_SetRelativeLocation` (`self.Plane`) (`KismetMathLibrary.VLerp` (0.0 0.0 0.0) (`|GetArrayItem` (`self.Location`) (`KismetMathLibrary.RandomInteger` 1)) _alpha) false false))
    (:`Finished`
      (if (`|EnumEquality` (`self.Direction`) "Backward")
        (`KismetSystemLibrary.Delay` (`|GetArrayItem` (`self.WaitDuration`) (`KismetMathLibrary.RandomInteger` 1)))
        (`self.Move`)
        (else
          (`KismetSystemLibrary.Delay` (`|GetArrayItem` (`self.WaitDuration`) (`KismetMathLibrary.RandomInteger` 1)))
          (goto _label :!via `Reverse`))))))

(event `/Game/Blueprints/Interfaces/BPI_Interact.Interact`
  (if (`self.AnimalReady`)
    (`/Game/Blueprints/GM_Base.UpdateMilk` (`self.GameMode`) 1)
    (`KismetSystemLibrary.PrintString` "GotMilk")
    (set `self.AnimalReady` false)
    (`KismetSystemLibrary.Delay` (`self.Duration`))
    (set `self.AnimalReady` true)
    (else
      (`KismetSystemLibrary.PrintString` "AnimalNotReady"))))

(fn `UserConstructionScript`
  (`parent.UserConstructionScript`))