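; Interactable farm animal that wanders back and forth and yields milk through GM_Base once fed.
; A looping MoveAnim timeline ping-pongs its trigger, plane and progress background toward Location, pausing by WaitDuration at each end.
; Interact plays FMOD audio, then either collects milk when ready or, if the sack is active, starts eating.
; Eating runs ProgressAnim at a Duration play rate, growing the progress bar until milk is ready.
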(event `self.ReceiveBeginPlay`
  (`parent.ReceiveBeginPlay`)
  (`self.Move`)
  (bind _asgm_base (cast `/Game/Blueprints/GM_Base` (`GameplayStatics.GetGameMode`)))
  (set `self.GameMode` _asgm_base))

(event `Move`
  (bind (_direction _alpha) (`Timeline|MoveAnim` :!via `PlayFromStart` :!label _label)
    (:`Update`
      (set `self.Direction` _direction)
      (`|ExecutionSequence`
        (:`then_1`
          (`SceneComponent.K2_SetRelativeLocation` (`self.Trigger`) (`KismetMathLibrary.VLerp` (0.0 0.0 0.0) (`self.Location`) _alpha) false false)
          (`SceneComponent.K2_SetRelativeLocation` (`self.Plane`) (`KismetMathLibrary.VLerp` (0.0 0.0 0.0) (`self.Location`) _alpha) false false)
          (`SceneComponent.K2_SetRelativeLocation` (`self.ProgressBK`) (`KismetMathLibrary.VLerp` (0.0 0.0 0.0) (`self.Location`) _alpha) false false))))
    (:`Finished`
      (if (`|EnumEquality` (`self.Direction`) "Backward")
        (`KismetSystemLibrary.Delay` (`|GetArrayItem` (`self.WaitDuration`) (`KismetMathLibrary.RandomInteger` 1)))
        (`self.Move`)
        (else
          (`KismetSystemLibrary.Delay` (`|GetArrayItem` (`self.WaitDuration`) (`KismetMathLibrary.RandomInteger` 1)))
          (goto _label :!via `Reverse`))))))

(event `self.Interact`
  (`FMODAudioComponent.Play` (`self.FMODAudio`))
  (if (`self.AnimalReady`)
    (`/Game/Blueprints/GM_Base.UpdateMilk` (`self.GameMode`) 1)
    (`KismetSystemLibrary.PrintString` "GotMilk")
    (set `self.AnimalReady` false)
    (`SceneComponent.SetRelativeScale3D` (`self.Progress`) (0.006983 0.0 0.946016))
    (elif (`/Game/Blueprints/GM_Base.SackActive` (`self.GameMode`))
      (if (not (`self.Eating`))
        (`self.Anim`))
      (else
        (`KismetSystemLibrary.PrintString` "AnimalNotReady")))))

(event `Anim`
  (set `self.AnimalReady` false)
  (set `self.Eating` true)
  (`TimelineComponent.SetPlayRate` (`self.ProgressAnim`) (`self.Duration`))
  (bind (_direction _alpha) (`Timeline|ProgressAnim` :!via `PlayFromStart`)
    (:`Update`
      (`SceneComponent.SetRelativeScale3D` (`self.Progress`) (`KismetMathLibrary.MakeVector` 0.006983 (`KismetMathLibrary.Lerp` 0.0 1.0 _alpha) 0.946016)))
    (:`Finished`
      (set `self.AnimalReady` true)
      (set `self.Eating` false))))

(fn `UserConstructionScript`
  (`parent.UserConstructionScript`))