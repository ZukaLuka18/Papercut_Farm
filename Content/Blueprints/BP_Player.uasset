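; Player character shown as a textured plane, with Enhanced Input movement, interaction and pause menu.
; Move input follows control yaw, sets facing flags and triggers delay-throttled footstep sounds.
; Tick reads velocity and those flags to cycle four-frame directional walk textures on a dynamic material, using Delay as the frame timer, or show an idle frame.
; Interact messages the first overlapping BPI_Interact actor; pause pushes WBP_PauseMenu through the HUD.
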(event `self.ReceiveBeginPlay`
  ;[1 1 1] Add mapping context
  (`EnhancedInputSubsystemInterface.AddMappingContext` (pcsubsystem `EnhancedInputLocalPlayerSubsystem` (`GameplayStatics.GetPlayerController` 0)) "/Game/Input/IMC_Player.IMC_Player" 0 (struct)))

(event `PlayStepSounds`
  (`KismetSystemLibrary.Delay` 0.4)
  (if (not (`self.AnimLoopEnded`))
    (`FMODBlueprintStatics.PlayEvent2D` "/Game/FMOD/Events/Steps.Steps")))

(event `EnhancedInput|/Game/Input/IA_Move`
  (params (ActionValue :type "Vector2D Structure") (ElapsedSeconds :type "Float (double-precision)") (TriggeredSeconds :type "Float (double-precision)") (InputAction :type "InputAction Object Reference" :default "/Game/Input/IA_Move.IA_Move"))
  (bind (_returnvalue_roll _returnvalue_pitch _returnvalue_yaw) (`KismetMathLibrary.BreakRotator` (`self.GetControlRotation`)))
  (bind (_returnvalue_roll_2 _returnvalue_pitch_2 _returnvalue_yaw_2) (`KismetMathLibrary.BreakRotator` (`self.GetControlRotation`)))
  (:`Triggered`
    (`self.PlayStepSounds`)
    (`self.CheckDirection1`)
    (`self.CheckDirection2`)
    ;[1 1 1] Movement
    (`self.AddMovementInput` (`KismetMathLibrary.NegateVector` (`KismetMathLibrary.GetForwardVector` (`KismetMathLibrary.MakeRotator` 0.0 0.0 _returnvalue_yaw_2))) ActionValue_X)
    (`self.AddMovementInput` (`KismetMathLibrary.NegateVector` (`KismetMathLibrary.GetRightVector` (`KismetMathLibrary.MakeRotator` 0.0 0.0 _returnvalue_yaw))) ActionValue_Y)))

(event `CheckDirection1`
  (if (> (`KismetMathLibrary.BreakVector2D` (stale `EnhancedInput|/Game/Input/IA_Move` ActionValue)) 0.0)
    (set `self.WalkingBackward` true)
    (set `self.WalkingForward` false)
    (elif (< (`KismetMathLibrary.BreakVector2D` (stale `EnhancedInput|/Game/Input/IA_Move` ActionValue)) 0.0)
      (set `self.WalkingForward` true)
      (set `self.WalkingBackward` false))))

(event `EnhancedInput|/Game/Input/IA_Interact`
  (params (ActionValue :type Boolean) (ElapsedSeconds :type "Float (double-precision)") (TriggeredSeconds :type "Float (double-precision)") (InputAction :type "InputAction Object Reference" :default "/Game/Input/IA_Interact.IA_Interact"))
  ;[1 1 1] Interact
  (:`Started`
    (for _array_element (`self.GetOverlappingActors` "/Script/Engine.Actor")
      (if (`KismetSystemLibrary.DoesImplementInterface` _array_element "/Game/Blueprints/Interfaces/BPI_Interact.BPI_Interact_C")
        (message `/Game/Blueprints/Interfaces/BPI_Interact.Interact` _array_element)
        (break)))))

(event `CheckDirection2`
  (if (> (`.Y` (`KismetMathLibrary.BreakVector2D` (stale `EnhancedInput|/Game/Input/IA_Move` ActionValue))) 0.0)
    (set `self.Right` true)
    (set `self.Left` false)
    (set `self.WalkingForward` false)
    ;[1 1 1] Interact
    (set `self.WalkingBackward` false)
    (elif (< (`.Y` (`KismetMathLibrary.BreakVector2D` (stale `EnhancedInput|/Game/Input/IA_Move` ActionValue))) 0.0)
      (set `self.Left` true)
      (set `self.Right` false)
      (set `self.WalkingForward` false)
      (set `self.WalkingBackward` false))))

(event `EnhancedInput|/Game/Input/IA_Pause`
  (params (ActionValue :type Boolean) (ElapsedSeconds :type "Float (double-precision)") (TriggeredSeconds :type "Float (double-precision)") (InputAction :type "InputAction Object Reference" :default "/Game/Input/IA_Pause.IA_Pause"))
  (bind _returnvalue (`GameplayStatics.GetPlayerController` 0))
  (:`Triggered`
    (bind _pushedwidget (message `/Game/Blueprints/Interfaces/BPI_PushWidgets.PushToGameplayStack` (`PlayerController.GetHUD` _returnvalue) "/Game/Blueprints/UI/WBP_PauseMenu.WBP_PauseMenu_C"))
    (`WidgetBlueprintLibrary.SetInputMode_UIOnlyEx` _returnvalue _pushedwidget)
    (set `PlayerController.bShowMouseCursor` true _returnvalue)))

(event `self.ReceiveTick`
  (params (DeltaSeconds :type "Float (single-precision)"))
  (`self.CheckVelocity`))

(event `CheckVelocity`
  (bind _returnvalue (not (`KismetMathLibrary.Vector_IsZero` (`MovementComponent.Velocity` (`self.CharacterMovement`)))))
  (if (and _returnvalue (`self.WalkingForward`))
    ;[1 1 1] forward
    (set `self.AnimLoopEnded` false)
    (`self.Animate` 0)
    (elif (and _returnvalue (`self.WalkingBackward`))
      ;[1 1 1] backward
      (set `self.AnimLoopEnded` false)
      (`self.Animate` 1)
      (elif (and _returnvalue (`self.Left`))
        ;[1 1 1] Left
        (set `self.AnimLoopEnded` false)
        (`self.Animate` 2)
        (elif (and _returnvalue (`self.Right`))
          ;[1 1 1] right
          (set `self.AnimLoopEnded` false)
          (`self.Animate` 3)
          (else
            ;[1 1 1] Stop
            (set `self.AnimLoopEnded` true)
            (`MaterialInstanceDynamic.SetTextureParameterValue` (`self.PlayerMaterial`) "Texture" "/Game/PNGS/Player/walk_s_2.walk_s_2")))))))

(event `SetIndex`
  (if (== (`self.IndexImage`) 0)
    (set `self.IndexImage` 1)
    (elif (== (`self.IndexImage`) 1)
      (set `self.IndexImage` 2)
      (elif (== (`self.IndexImage`) 2)
        (set `self.IndexImage` 3)
        (elif (== (`self.IndexImage`) 3)
          (set `self.IndexImage` 0))))))

(event `Animate`
  (params (Direction :type Integer))
  (`KismetSystemLibrary.Delay` 0.2)
  (if (not (`self.AnimLoopEnded`))
    (`MaterialInstanceDynamic.SetTextureParameterValue` (`self.PlayerMaterial`) "Texture" (`|GetArrayItem` (select `int` Direction :`0` (`self.WalkForward`) :`1` (`self.WalkBackward`) :`2` (`self.WalkLeft`) :`3` (`self.WalkRight`)) (`self.IndexImage`)))
    (`self.SetIndex`)))

(fn `UserConstructionScript`
  (bind _returnvalue (`PrimitiveComponent.CreateDynamicMaterialInstance` (`self.Plane`) 0 "/Game/Material/M_Texture_Player.M_Texture_Player" "None"))
  (set `self.PlayerMaterial` _returnvalue))