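; Sales stand interactable where the player turns in the active quest order.
; On BeginPlay it caches GM_Base; Interact acts only when CanComit is set, clearing quest state and showing the HUD's back-to-quest-stack message.
; A nested branch chain picks the flagged good (Trunkblume, Stingsquach, Milk or Goat) and subtracts the order amount chosen by the NeedCorrect flags from its GameMode count.
; It then resets that good's flags and all Correct flags.
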(event `self.ReceiveBeginPlay`
  (`parent.ReceiveBeginPlay`)
  (bind _asgm_base (cast `/Game/Blueprints/GM_Base` (`GameplayStatics.GetGameMode`)))
  (set `self.GameMode` _asgm_base))

(event `/Game/Blueprints/Interfaces/BPI_Interact.Interact`
  (bind _gamemode (`self.GameMode`))
  (bind _gamemode_2 (`self.GameMode`))
  (bind _stingsquach (`/Game/Blueprints/GM_Base.Stingsquach` _gamemode))
  (bind _milk (`/Game/Blueprints/GM_Base.Milk` _gamemode))
  (bind _goat (`/Game/Blueprints/GM_Base.Goat` _gamemode))
  (bind _needcorrect2 (`/Game/Blueprints/GM_Base.NeedCorrect2` _gamemode))
  (bind _needcorrect3 (`/Game/Blueprints/GM_Base.NeedCorrect3` _gamemode))
  (bind _amountorder1 (`/Game/Blueprints/GM_Base.AmountOrder1` _gamemode))
  (bind _amountorder2 (`/Game/Blueprints/GM_Base.AmountOrder2` _gamemode))
  (bind _amountorder3 (`/Game/Blueprints/GM_Base.AmountOrder3` _gamemode))
  (bind _trunkblume (`/Game/Blueprints/GM_Base.Trunkblume` _gamemode))
  (if (`/Game/Blueprints/GM_Base.CanComit` _gamemode_2)
    (`KismetSystemLibrary.PrintString` "Hello")
    (set `/Game/Blueprints/GM_Base.QuestOn` false _gamemode_2)
    (set `/Game/Blueprints/GM_Base.CanComit` false _gamemode_2)
    (message `/Game/Blueprints/Interfaces/BPI_PushWidgets.BackToQuestStack` (`PlayerController.GetHUD` (`GameplayStatics.GetPlayerController` 0)))
    (set `/Game/Blueprints/GM_Base.QuestAmount` 0 _gamemode)
    (`|ExecutionSequence`
      (:`then_0`
        (if (`/Game/Blueprints/GM_Base.ItsTrunk` _gamemode)
          (if _needcorrect2
            (set `/Game/Blueprints/GM_Base.Trunkblume` (- _trunkblume _amountorder2) _gamemode)
            (set `/Game/Blueprints/GM_Base.ItsTrunk` false _gamemode)
            (set `/Game/Blueprints/GM_Base.NeedCorrect2` false _gamemode)
            (elif _needcorrect3
              (set `/Game/Blueprints/GM_Base.Trunkblume` (- _trunkblume _amountorder3) _gamemode)
              (set `/Game/Blueprints/GM_Base.ItsTrunk` false _gamemode)
              (set `/Game/Blueprints/GM_Base.NeedCorrect3` false _gamemode)
              (else
                (set `/Game/Blueprints/GM_Base.Trunkblume` (- _trunkblume _amountorder1) _gamemode)
                (set `/Game/Blueprints/GM_Base.ItsTrunk` false _gamemode))))
          (elif (`/Game/Blueprints/GM_Base.ItsSting` _gamemode)
            (if _needcorrect2
              (set `/Game/Blueprints/GM_Base.Stingsquach` (- _stingsquach _amountorder2) _gamemode)
              (set `/Game/Blueprints/GM_Base.ItsSting` false _gamemode)
              (set `/Game/Blueprints/GM_Base.NeedCorrect2` false _gamemode)
              (elif _needcorrect3
                (set `/Game/Blueprints/GM_Base.Stingsquach` (- _stingsquach _amountorder3) _gamemode)
                (set `/Game/Blueprints/GM_Base.ItsSting` false _gamemode)
                (set `/Game/Blueprints/GM_Base.NeedCorrect3` false _gamemode)
                (else
                  (set `/Game/Blueprints/GM_Base.Stingsquach` (- _stingsquach _amountorder1) _gamemode)
                  (set `/Game/Blueprints/GM_Base.ItsSting` false _gamemode))))
            (elif (`/Game/Blueprints/GM_Base.ItsMilk` _gamemode)
              (if _needcorrect2
                (set `/Game/Blueprints/GM_Base.Milk` (- _milk _amountorder2) _gamemode)
                (set `/Game/Blueprints/GM_Base.ItsMilk` false _gamemode)
                (set `/Game/Blueprints/GM_Base.NeedCorrect2` false _gamemode)
                (elif _needcorrect3
                  (set `/Game/Blueprints/GM_Base.Milk` (- _milk _amountorder3) _gamemode)
                  (set `/Game/Blueprints/GM_Base.ItsMilk` false _gamemode)
                  (set `/Game/Blueprints/GM_Base.NeedCorrect3` false _gamemode)
                  (else
                    (set `/Game/Blueprints/GM_Base.Milk` (- _milk _amountorder1) _gamemode)
                    (set `/Game/Blueprints/GM_Base.ItsMilk` false _gamemode))))
              (elif (`/Game/Blueprints/GM_Base.ItsGoat` _gamemode)
                (if _needcorrect2
                  (set `/Game/Blueprints/GM_Base.Goat` (- _goat _amountorder2) _gamemode)
                  (set `/Game/Blueprints/GM_Base.ItsGoat` false _gamemode)
                  (set `/Game/Blueprints/GM_Base.NeedCorrect2` false _gamemode)
                  (elif _needcorrect3
                    (set `/Game/Blueprints/GM_Base.Goat` (- _goat _amountorder3) _gamemode)
                    (set `/Game/Blueprints/GM_Base.ItsGoat` false _gamemode)
                    (set `/Game/Blueprints/GM_Base.NeedCorrect3` false _gamemode)
                    (else
                      (set `/Game/Blueprints/GM_Base.Goat` (- _goat _amountorder1) _gamemode)
                      (set `/Game/Blueprints/GM_Base.ItsGoat` false _gamemode)))))))))
      (:`then_1`
        (set `/Game/Blueprints/GM_Base.Correct1` false _gamemode)
        (set `/Game/Blueprints/GM_Base.Correct2` false _gamemode)
        (set `/Game/Blueprints/GM_Base.Correct3` false _gamemode)))))

(fn `UserConstructionScript`
  (`parent.UserConstructionScript`))