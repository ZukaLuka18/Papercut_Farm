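; BP_Structures_Grass is a grass structure actor that displays a configurable texture on a Plane component.
; Its construction script creates a dynamic instance of M_Texture_Grass on the plane and stores it as Material, then runs the parent's construction script.
; BeginPlay runs the parent logic, then writes the Texture variable into the material's "Texture" parameter.
; Overlap and Tick events are disabled stubs.
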(event `self.ReceiveBeginPlay`
  (`parent.ReceiveBeginPlay`)
  (`MaterialInstanceDynamic.SetTextureParameterValue` (`self.Material`) "Texture" (`self.Texture`)))

(fn `UserConstructionScript`
  (bind _returnvalue (`PrimitiveComponent.CreateDynamicMaterialInstance` (`self.Plane`) 0 "/Game/Material/M_Texture_Grass.M_Texture_Grass" "None"))
  (set `self.Material` _returnvalue)
  (`parent.UserConstructionScript`))