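; Interactable quest board that opens a quest selection widget when the player interacts with it.
; Interact pushes WBP_QuestBoard onto the HUD's quest board stack, then switches to UI-only input focused on it and shows the mouse cursor.
; A Shuffle event randomizes Quests and appends the first three to RandomQuests for a unique selection, though nothing in this graph calls it.
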(event `self.ReceiveBeginPlay`
  (`parent.ReceiveBeginPlay`))

(event `Shuffle2`
  (`KismetArrayLibrary.Array_Shuffle` (`self.Quests`)))

(event `Shuffle`
  ;[1 1 1] create unique quest selection
  (`KismetArrayLibrary.Array_Shuffle` (`self.Quests`))
  (for (_array_element _array_index) (`self.Quests`) :!label _label
    (if (== _array_index 3)
      (`self.Break`)
      (else
        (`KismetArrayLibrary.Array_Add` (`self.RandomQuests`) _array_element)))))

(event `Break`
  ;[1 1 1] create unique quest selection
  (goto _label :!via `Break`))

(event `/Game/Blueprints/Interfaces/BPI_Interact.Interact`
  (bind _returnvalue (`GameplayStatics.GetPlayerController` 0))
  ;[1 1 1] Show widget on interact
  (bind _pushedwidget (message `/Game/Blueprints/Interfaces/BPI_PushWidgets.PushToQuestBoardStack` (`PlayerController.GetHUD` _returnvalue) "/Game/Blueprints/UI/WBP_QuestBoard.WBP_QuestBoard_C"))
  (bind _output_get (set `self.Pushed Widget` _pushedwidget))
  (`WidgetBlueprintLibrary.SetInputMode_UIOnlyEx` _returnvalue _output_get "DoNotLock" true)
  (set `PlayerController.bShowMouseCursor` true _returnvalue))

(fn `UserConstructionScript`
  (`parent.UserConstructionScript`))